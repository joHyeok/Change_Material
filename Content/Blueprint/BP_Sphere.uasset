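; BP_Sphere is a clickable actor with a Sphere and a Cube component that each respond to mouse clicks.
; Sphere clicks are delegated to a SphereLogic object, which the game mode assigns through SetSphereLogic and which can retrieve the mesh through GetSphereMesh.
; Cube clicks are handled locally, advancing a wrapping index that cycles the cube's material through gold, copper and lake water.
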(event OnClicked(Sphere)
  (params (TouchedComponent :type Primitive%20Component%20Object%20Reference) (ButtonPressed :type Key%20Structure :default "None"))
  ;[1 1 1] 스피어를 클릭하면 SphereLogicBP의 Click Sphere 이벤트 발생
  (Default|ClickSphere (Variables|Default|GetSphereLogic)))

(event OnClicked(Cube)
  (params (TouchedComponent :type Primitive%20Component%20Object%20Reference) (ButtonPressed :type Key%20Structure :default "None"))
  ;[1 1 1] 큐브를 클릭하면 머티리얼이 바뀐다.
  (Variables|Default|SetMaterialNumber (Math|Integer|%(Integer) (+ (Variables|Default|GetMaterialNumber) 1) 3))
  (CallFunction|SetMaterial))

(event Custom|SetMaterial
  ;[1 1 1] 큐브의 머티리얼 변경
  (switch int (Variables|Default|GetMaterialNumber)
    (:0
      (Rendering|Material|SetMaterial (Variables|Default|GetCube) 0 "/Game/StarterContent/Materials/M_Metal_Gold.M_Metal_Gold"))
    (:1
      (Rendering|Material|SetMaterial (Variables|Default|GetCube) 0 "/Game/StarterContent/Materials/M_Metal_Copper.M_Metal_Copper"))
    (:2
      (Rendering|Material|SetMaterial (Variables|Default|GetCube) 0 "/Game/StarterContent/Materials/M_Water_Lake.M_Water_Lake"))))

(event EventBeginPlay)

(event Collision|EventActorBeginOverlap
  (params (OtherActor :type Actor%20Object%20Reference)))

(event EventTick
  (params (DeltaSeconds :type Float%20%28single-precision%29)))

(fn ConstructionScript)

(fn SetSphereLogic
  (params (SphereLogic :type BP%20Sphere%20Logic%20Object%20Reference))
  ;[1 1 1] 게임모드에서 SphereLogicBP 할당
  (Variables|Default|SetSphereLogic SphereLogic))

(fn GetSphereMesh
  ;[1 1 1] LogicBP에서 스피어의 메쉬 가져가기
  (return (Variables|Default|GetSphere)))