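; BP_BoxMetarialLogic is an actor that cycles the material on a group of box actors.
; IniBoxList stores the boxes passed in, and each ClickActor call advances a wrapping counter to select one of five brick, ground, metal or rock materials.
; SetMaterial then applies that material to slot 0 of every listed box's mesh.
; Its own event graph is empty, so other Blueprints must drive it.
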(event EventBeginPlay)

(event Collision|EventActorBeginOverlap
  (params (OtherActor :type Actor%20Object%20Reference)))

(event EventTick
  (params (DeltaSeconds :type Float%20%28single-precision%29)))

(fn ConstructionScript)

(fn SetMaterial
  (params (Material :type Material%20Object%20Reference))
  ;[1 1 1] 박스의 Mesh를 가져와서 머티리얼 Set하기
  (for _array_element (Variables|Default|GetBoxList)
    (bind _box_mesh_component (Default|GetBoxMesh _array_element))
    (Rendering|Material|SetMaterial _box_mesh_component 0 Material)))

(fn ClickActor
  (bind _output_get (Variables|Default|SetMaterialNumber (Math|Integer|%(Integer) (+ (Variables|Default|GetMaterialNumber) 1) (Variables|Default|GetMaxNumber))))
  (switch int _output_get
    (:0
      ;[1 1 1] 머티리얼 교체
      (CallFunction|SetMaterial "/Game/StarterContent/Materials/M_Brick_Clay_New.M_Brick_Clay_New"))
    (:1
      (CallFunction|SetMaterial "/Game/StarterContent/Materials/M_Ground_Moss.M_Ground_Moss"))
    (:2
      (CallFunction|SetMaterial "/Game/StarterContent/Materials/M_Metal_Copper.M_Metal_Copper"))
    (:3
      (CallFunction|SetMaterial "/Game/StarterContent/Materials/M_Metal_Steel.M_Metal_Steel"))
    (:4
      (CallFunction|SetMaterial "/Game/StarterContent/Materials/M_Rock_Basalt.M_Rock_Basalt"))))

(fn IniBoxList
  (params (BoxList :type Array%20of%20BP%20Box%20Object%20References))
  (Variables|Default|SetBoxList BoxList))