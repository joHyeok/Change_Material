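; BP_SphereLogic changes the material of a group of spheres on each click.
; SetSphereList stores the sphere array, which the game mode is meant to assign.
; ClickSphere advances a wrapping counter to pick steel, gold or copper, then SetMaterial applies it to every sphere's mesh.
; Its event graph is empty, so all work runs through these externally called functions.
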(event EventBeginPlay)

(event Collision|EventActorBeginOverlap
  (params (OtherActor :type Actor%20Object%20Reference)))

(event EventTick
  (params (DeltaSeconds :type Float%20%28single-precision%29)))

(fn ConstructionScript)

(fn ClickSphere
  ;[1 1 1] 클릭 횟수에 따라 다른 머티리얼 적용
  (bind _output_get (Variables|Default|SetMaterial%20Number (Math|Integer|%(Integer) (+ (Variables|Default|GetMaterial%20Number) 1) (Variables|Default|GetMax%20Material%20Number))))
  (switch int _output_get
    (:0
      (CallFunction|SetMaterial "/Game/StarterContent/Materials/M_Metal_Steel.M_Metal_Steel"))
    (:1
      (CallFunction|SetMaterial "/Game/StarterContent/Materials/M_Metal_Gold.M_Metal_Gold"))
    (:2
      (CallFunction|SetMaterial "/Game/StarterContent/Materials/M_Metal_Copper.M_Metal_Copper"))))

(fn SetMaterial
  (params (Material :type Material%20Object%20Reference))
  ;[1 1 1] 스피어의 Mesh를 가져와서 머티리얼 변경
  (for _array_element (Variables|Default|GetSphereList)
    (bind _sphere_mesh (Default|GetSphereMesh _array_element))
    (Rendering|Material|SetMaterial _sphere_mesh 0 Material)))

(fn SetSphereList
  (params (SphereList :type Array%20of%20BP%20Sphere%20Object%20References))
  ;[1 1 1] 게임모드에서 스피어 배열 할당
  (Variables|Default|SetSphereList SphereList))