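; BP_GM is a manager Blueprint that wires the level's BP_Sphere actors to a shared BP_SphereLogic actor at BeginPlay.
; A sequence finds the logic actor, gathers all spheres and passes that list to it through SetSphereList.
; It then gives each sphere a reference back to the logic actor through SetSphereLogic, linking both sides.
; Tick and the construction script are empty.
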(event EventBeginPlay
  (Utilities|FlowControl|Sequence
    (:then_0
      ;[1 1 1] Sphere Logic bp 변수 생성
      (bind _returnvalue (Actor|GetActorOfClass "/Game/Blueprint/BP_SphereLogic.BP_SphereLogic_C"))
      (Variables|Default|SetSphere%20Logic%20BP _returnvalue))
    (:then_1
      ;[1 1 1] Sphere들을 가져와서 SphereLogicBP에 초기화
      (bind _outactors (Actor|GetAllActorsOfClass "/Game/Blueprint/BP_Sphere.BP_Sphere_C"))
      (bind _output_get (Variables|Default|SetSphereList _outactors))
      (Default|SetSphereList (Variables|Default|GetSphere%20Logic%20BP) _output_get))
    (:then_2
      ;[1 1 1] Sphere들에 SphereLogicBP추가
      (for _array_element (Variables|Default|GetSphereList)
        (Default|SetSphereLogic _array_element (Variables|Default|GetSphere%20Logic%20BP))))))

(event EventTick
  (params (DeltaSeconds :type Float%20%28single-precision%29)))

(fn ConstructionScript)